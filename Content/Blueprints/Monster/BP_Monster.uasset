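; BP_Monster is an enemy monster Blueprint that attacks the player and removes itself after death.
; Tick watches Hp and, at zero or below, stops the BP_MonsterController brain logic, then destroys the actor after a delay.
; Attack snaps rotation toward the BP_Player found in the level, plays an effort sound, and briefly pulses the Attack flag on ABP_Monster to drive animation.
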(event `self.ReceiveTick`
  (params (DeltaSeconds :type "Float (single-precision)"))
  (if (<= (`self.Hp`) 0.0)
    (bind _asbp_monster_controller (cast `/Game/Blueprints/Monster/BP_MonsterController` (`self.GetController`)))
    (`BrainComponent.StopLogic` (`AIController.BrainComponent` _asbp_monster_controller) "")
    (`KismetSystemLibrary.Delay` 10.0)
    (`self.K2_DestroyActor`)))

(event `Attack`
  (bind _returnvalue (`self.K2_GetActorLocation`))
  (bind _returnvalue_2 (`GameplayStatics.GetActorOfClass` "/Game/Blueprints/BP_Player.BP_Player_C"))
  (`self.K2_SetActorRotation` (`KismetMathLibrary.FindLookAtRotation` _returnvalue (`self.K2_GetActorLocation` _returnvalue_2)))
  (bind _asabp_monster (cast `/Game/Animations/Monster/ABP_Monster` (`SkeletalMeshComponent.GetAnimInstance` (`self.Mesh`))))
  (set `/Game/Animations/Monster/ABP_Monster.bAttack` true _asabp_monster)
  (`GameplayStatics.PlaySoundAtLocation` "/Game/Sounds/Rampage_Effort_Ability_Primary_Edited.Rampage_Effort_Ability_Primary_Edited" _returnvalue (struct) 1.0 1.0 0.0 null null null null)
  (`KismetSystemLibrary.Delay` 0.5)
  (set `/Game/Animations/Monster/ABP_Monster.bAttack` false _asabp_monster))

(fn `UserConstructionScript`)