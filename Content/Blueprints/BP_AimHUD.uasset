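; BP_AimHUD is a HUD Blueprint that draws an aiming crosshair near the middle of the screen.
; BeginPlay keeps the crosshair hidden through a short startup delay, then sets a visibility flag.
; While that flag is set, DrawHUD draws the masked crosshair texture each frame, positioned from the viewport size with a fixed upward offset from center.
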(event `self.ReceiveBeginPlay`
  (set `self.bIsCrosshairVisible` false)
  (`KismetSystemLibrary.Delay` 5.0)
  (set `self.bIsCrosshairVisible` true))

(event `self.ReceiveDrawHUD`
  (params (SizeX :type Integer) (SizeY :type Integer))
  (if (`self.bIsCrosshairVisible`)
    (`self.DrawTexture` "/Game/Assets/CrossHair.CrossHair" (`KismetMathLibrary.Conv_IntToDouble` (- (/ SizeX 2) 32)) (`KismetMathLibrary.Conv_IntToDouble` (- (- (/ SizeY 2) 32) 30)) 64.0 64.0 0.0 0.0 1.0 1.0 (struct :`R` 1.0 :`G` 1.0 :`B` 1.0 :`A` 1.0) "BLEND_Masked" 0.5)))

(fn `UserConstructionScript`)